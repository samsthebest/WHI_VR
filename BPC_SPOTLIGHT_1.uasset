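; Interactable spotlight Blueprint that the game can switch on and off.
; The direct interact event and the external switch event run the same toggle, flipping SpotLight visibility and tracking state in LIGHTOFF.
; Both events do nothing when EXTERNALSWITCH is set, and the construction script only calls its parent.
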(event EventInteractwithObject
  (if (not (Variables|Default|GetEXTERNAL_SWITCH))
    (if (Variables|Default|GetLIGHT%20OFF)
      (Rendering|SetVisibility (Variables|Default|GetSpotLight) true false)
      (Variables|Default|SetLIGHT%20OFF false)
      (else
        (Rendering|SetVisibility (Variables|Default|GetSpotLight) false false)
        (Variables|Default|SetLIGHT%20OFF true)))))

(event EventInteractExternalSwitch
  (if (not (Variables|Default|GetEXTERNAL_SWITCH))
    (if (Variables|Default|GetLIGHT%20OFF)
      (Rendering|SetVisibility (Variables|Default|GetSpotLight) true false)
      (Variables|Default|SetLIGHT%20OFF false)
      (else
        (Rendering|SetVisibility (Variables|Default|GetSpotLight) false false)
        (Variables|Default|SetLIGHT%20OFF true)))))

(fn ConstructionScript
  (|CallParentFunction))